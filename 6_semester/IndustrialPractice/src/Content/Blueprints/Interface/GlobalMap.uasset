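; GlobalMap is an actor Blueprint that sets up the interface for the global map when play begins.
; BeginPlay shows the mouse cursor, then creates the BP_GlobalMap and BP_LevelCard widgets and adds both to the viewport.
; It also queries all BP_MapActor actors without using the result.
; Disconnected leftover nodes for camera blending, actor spawning and widget creation never run.
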(event `self.ReceiveBeginPlay`
  (set `PlayerController.bShowMouseCursor` true (`GameplayStatics.GetPlayerController` 0))
  (`GameplayStatics.GetAllActorsOfClass` "/Game/Blueprints/Interface/BP_MapActor.BP_MapActor_C")
  (bind _returnvalue (`|CreateWidget` "/Game/Blueprints/Interface/BP_GlobalMap.BP_GlobalMap_C"))
  (bind _returnvalue_2 (`|CreateWidget` "/Game/Blueprints/Interface/BP_LevelCard.BP_LevelCard_C"))
  (`UserWidget.AddToViewport` _returnvalue 0)
  (`UserWidget.AddToViewport` _returnvalue_2 0))

(fn `UserConstructionScript`)