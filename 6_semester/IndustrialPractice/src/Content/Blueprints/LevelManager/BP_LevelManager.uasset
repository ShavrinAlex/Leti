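; Level manager that runs enemy waves, holds Money and Life, and pauses the game when Life reaches zero, checked on Tick.
; BeginPlay creates the level widget, initializes the node graph and spawns a MissionActor as the wave timer.
; Each wave expiry runs a delayed-loop macro that staggers enemy spawns.
; Each AI mob spawns at the graph's best start node, offset to its best up, middle or down sub-node.
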(event `self.ReceiveBeginPlay`
  (set `self.is_game_over` false)
  (`self.CreateWidget`)
  (`KismetSystemLibrary.Delay` 0.2)
  (`self.init_graph`)
  (bind _returnvalue (`|SpawnActorFromClass` "/Script/TowerDefense.MissionActor" (`KismetMathLibrary.MakeTransform` (0.0 0.0 0.0)) "Undefined" "MultiplyWithRoot" null null))
  (bind _output_get (set `self.WaveTimer` _returnvalue))
  (add `MissionActor.OnWaveExpired` _output_get (delegate `WaveExpiredevent_Custom`)))

(event `WaveExpiredevent_Custom`
  (`self.ForLoopWithDelay` 0 3 :!label _label
    (:`LoopBody`
      (`self.SetEnemyMob`))
    (:`ToDelay`
      (`KismetSystemLibrary.Delay` 2.0)
      (goto _label :!via `Delay`))))

(event `self.ReceiveTick`
  (params (DeltaSeconds :type "Float (single-precision)"))
  (if (== (`self.life`) 0)
    (bind _output_get (set `self.is_game_over` true))
    (`GameplayStatics.SetGamePaused` _output_get)))

(fn `CreateWidget`
  (bind _returnvalue (`GameplayStatics.GetPlayerController` 0))
  (set `PlayerController.bEnableClickEvents` true _returnvalue)
  (bind _returnvalue_2 (`|CreateWidget` "/Game/Blueprints/LevelManager/WBP_LevelManager.WBP_LevelManager_C" _returnvalue))
  (bind _output_get (set `self.level_menu_ref` _returnvalue_2))
  (`UserWidget.AddToViewport` _output_get 0))

(fn `SetEnemyMob`
  (locals (SubNodeLocation :type "Vector Structure"))
  (bind _subnodelocation (`local.SubNodeLocation`))
  (bind _returnvalue (`RoadGraph.get_best_start` (`self.graph`)))
  (set `local.SubNodeLocation` (`RoadNode.location` _returnvalue))
  (bind _returnvalue_2 (`RoadNode.get_best_sub_node` _returnvalue))
  (switch `SubNode` _returnvalue_2
    (:`UP`
      (set `local.SubNodeLocation` (+ _subnodelocation (0.0 100.0 0.0))))
    (:`MIDDLE`
      _)
    (:`DOWN`
      (set `local.SubNodeLocation` (- _subnodelocation (0.0 100.0 0.0)))))
  (bind _returnvalue_3 (`AIBlueprintHelperLibrary.SpawnAIFromClass` "/Game/Blueprints/Mobs/EnemyMobs/BP_EnemyMob.BP_EnemyMob_C" "/Game/Blueprints/Mobs/EnemyMobs/BT_EnemyMob.BT_EnemyMob" (`local.SubNodeLocation`) (struct) false null))
  (bind _asbp_enemy_mob (cast `/Game/Blueprints/Mobs/EnemyMobs/BP_EnemyMob` _returnvalue_3))
  (set `EnemyMob.current_node` _returnvalue _asbp_enemy_mob)
  (set `EnemyMob.sub_node` _returnvalue_2 _asbp_enemy_mob))

(fn `UserConstructionScript`
  (set `self.money` 1000))