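; BP_EnemyMob is an enemy character with health that can fight a target and drops money when killed.
; Tick polls health; at zero or below it disables movement, stops the AI brain and, after a short delay, spawns BP_Money slightly below its location and destroys itself.
; GetDamage reduces health and prints it, while FightWith halts movement and deals fixed damage to the passed-in target.
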(event `self.ReceiveBeginPlay`)

(event `self.ReceiveTick`
  (params (DeltaSeconds :type "Float (single-precision)"))
  (`self.UpdateAlive`)
  (if (`self.IsDead`)
    (`CharacterMovementComponent.DisableMovement` (`self.CharacterMovement`))
    (`BrainComponent.StopLogic` (`AIController.BrainComponent` (`AIBlueprintHelperLibrary.GetAIController` self)) "death")
    (`KismetSystemLibrary.Delay` 1.0)
    (`self.Death`)))

(fn `Death`
  (`self.SpawnMoney`)
  (`self.K2_DestroyActor`))

(fn `FightWith`
  (params (NewParam :type "/Game/Blueprints/Mobs/GuardianMobs/BP_GuardianMob Object Reference"))
  (`MovementComponent.StopMovementImmediately` (`self.CharacterMovement`))
  (`/Game/Blueprints/Mobs/GuardianMobs/BP_GuardianMob.GetDamage` NewParam 30))

(fn `GetDamage`
  (params (Damage :type Integer))
  (bind _output_get (set `self.Health` (`KismetMathLibrary.FTrunc` (- (`self.Health`) Damage))))
  (`KismetSystemLibrary.PrintString` (`KismetStringLibrary.Concat_StrStr` "Enemy " (`KismetStringLibrary.Conv_IntToString` _output_get))))

(fn `SpawnMoney`
  (bind (_returnvalue_x _returnvalue_y _returnvalue_z) (`KismetMathLibrary.BreakVector` (`self.K2_GetActorLocation`)))
  (`|SpawnActorFromClass` "/Game/Blueprints/Money/BP_Money.BP_Money_C" (`KismetMathLibrary.MakeTransform` (`KismetMathLibrary.MakeVector` _returnvalue_x _returnvalue_y (- _returnvalue_z 20.0))) "Undefined" "MultiplyWithRoot" null null))

(fn `UpdateAlive`
  (set `self.IsDead` (<= (`self.Health`) 0)))

(fn `UserConstructionScript`)