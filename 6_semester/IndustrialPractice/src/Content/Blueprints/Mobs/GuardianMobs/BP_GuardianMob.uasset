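; BP_GuardianMob is an AI-controlled guardian enemy with a sprite, health and death handling.
; On BeginPlay it sets a default directionality and actor rotation, and every tick it locks the sprite to a fixed world rotation.
; GetDamage lowers health and prints it for debugging.
; Tick polls health, and at zero or below it disables movement, stops the AI brain and destroys the actor after a short delay.
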(event `self.ReceiveBeginPlay`
  (`self.SetDefaultDirectionality`))

(event `self.ReceiveTick`
  (params (DeltaSeconds :type "Float (single-precision)"))
  (`self.UpdateSpriteRotation`)
  (`self.UpdateAlive`)
  (if (`self.IsDead`)
    (`CharacterMovementComponent.DisableMovement` (`self.CharacterMovement`))
    (`BrainComponent.StopLogic` (`AIController.BrainComponent` (`AIBlueprintHelperLibrary.GetAIController` self)) "death")
    (`KismetSystemLibrary.Delay` 1.0)
    (`self.Death`)))

(fn `Death`
  (`self.K2_DestroyActor`))

(fn `GetDamage`
  (params (Damage :type Integer))
  (bind _output_get (set `self.Health` (`KismetMathLibrary.FTrunc` (- (`self.Health`) Damage))))
  (`KismetSystemLibrary.PrintString` (`KismetStringLibrary.Concat_StrStr` "Guard " (`KismetStringLibrary.Conv_IntToString` _output_get))))

(fn `SetDefaultDirectionality`
  (set `self.Directionality` (-1.0 0.0))
  (`self.K2_SetActorRotation` (struct :`Roll` -1.0)))

(fn `UpdateAlive`
  (set `self.IsDead` (<= (`self.Health`) 0)))

(fn `UpdateSpriteRotation`
  (bind _sprite (`self.Sprite`))
  (if (!= (`SceneComponent.K2_GetComponentRotation` _sprite) (struct :`Yaw` 180.0 :`Roll` -90.0))
    (`SceneComponent.K2_SetWorldRotation` _sprite (struct :`Yaw` 180.0 :`Roll` -90.0) false false)))

(fn `UserConstructionScript`)