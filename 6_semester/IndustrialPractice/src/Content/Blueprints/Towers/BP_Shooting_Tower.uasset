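; Tower actor that automatically shoots at the nearest living BP_EnemyMob within its visibility radius.
; Tick counts frames up to a shoot delay, then calls FindMob each frame until a target appears, fires and resets the counter.
; FindMob scans all enemy actors by distance from the tower mesh.
; Shoot spawns a BP_Shot at a fixed height above the tower's XY, passing it target, speed and damage.
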(event `self.ReceiveTick`
  (params (DeltaSeconds :type "Float (single-precision)"))
  (if (== (`self.shoot_counter`) (`self.shoot_delay`))
    (bind (_nearest_mob _nearest_mob_distance _nearest_mob_location) (`self.FindMob`))
    (if (`KismetSystemLibrary.IsValid` _nearest_mob)
      (`self.Shoot` _nearest_mob _nearest_mob_location)
      (set `self.shoot_counter` 0))
    (else
      (`/Engine/EditorBlueprintResources/StandardMacros.IncrementInt` (`self.shoot_counter`)))))

(fn `FindMob`
  (returns (nearest_mob :type "/Game/Blueprints/Mobs/EnemyMobs/BP_EnemyMob Object Reference") (nearest_mob_distance :type "Float (double-precision)") (nearest_mob_location :type "Vector Structure"))
  (set `self.tower_location` (`SceneComponent.K2_GetComponentLocation` (`self.Mesh`)))
  (set `self.nearest_mob` null)
  (set `self.nearest_mob_distance` 10000000.0)
  (set `self.nearest_mob_location` (0.0 0.0 0.0))
  (bind _outactors (`GameplayStatics.GetAllActorsOfClass` "/Game/Blueprints/Mobs/EnemyMobs/BP_EnemyMob.BP_EnemyMob_C"))
  (for _array_element _outactors
    (if (`KismetSystemLibrary.IsValid` _array_element)
      (bind _returnvalue (`self.K2_GetActorLocation` _array_element))
      (bind _returnvalue_2 (`KismetMathLibrary.Vector_Distance` _returnvalue (`self.tower_location`)))
      (if (and (and (< _returnvalue_2 (`self.nearest_mob_distance`)) (not (`Mob.IsDead` _array_element))) (< _returnvalue_2 (`self.visibility_radius`)))
        (set `self.nearest_mob_location` _returnvalue)
        (set `self.nearest_mob_distance` _returnvalue_2)
        (set `self.nearest_mob` _array_element))))
  (return (`self.nearest_mob`) (`self.nearest_mob_distance`) (`self.nearest_mob_location`)))

(fn `Shoot`
  (params (Mob :type "/Game/Blueprints/Mobs/EnemyMobs/BP_EnemyMob Object Reference") (Location :type "Vector Structure"))
  (bind _returnvalue (`|SpawnActorFromClass` "/Game/Blueprints/Towers/BP_Shot.BP_Shot_C" (`KismetMathLibrary.MakeTransform` (`KismetMathLibrary.MakeVector` (.x (`self.tower_location`)) (.y (`self.tower_location`)) 40.0)) "AlwaysSpawn" "MultiplyWithRoot" null null))
  (if (`KismetSystemLibrary.IsValid` Mob)
    (`/Game/Blueprints/Towers/BP_Shot.SetShotParams` _returnvalue 25 Mob Location 35 (`SceneComponent.K2_GetComponentLocation` (`self.CapsuleComponent`)))))

(fn `UserConstructionScript`
  (`parent.UserConstructionScript`)
  (set `self.shoot_delay` 50)
  (set `self.visibility_radius` 500))