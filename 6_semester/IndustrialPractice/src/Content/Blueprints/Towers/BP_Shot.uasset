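; Tower projectile that flies at an enemy mob, damages the first BP_EnemyMob its box overlaps, then destroys itself.
; SetShotParams predicts an intercept point from the mob's velocity and flight time, then MakeOffset turns it into a fixed XY step.
; Tick applies that step per frame without delta-time scaling or homing, keeping Z constant, and destroys the shot if the target becomes invalid.
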(event `self.ReceiveTick`
  (params (DeltaSeconds :type "Float (single-precision)"))
  (`self.Go To Mob`))

(event `self.Box.OnComponentBeginOverlap`
  (params (OverlappedComponent :type "PrimitiveComponent Object Reference") (OtherActor :type "Actor Object Reference") (OtherComp :type "PrimitiveComponent Object Reference") (OtherBodyIndex :type Integer) (bFromSweep :type Boolean) (SweepResult :type "HitResult Structure (by ref)"))
  (`self.TouchEnemyMobHandler` OtherActor))

(fn `CalculateMobLocation`
  (params (`target point` :type "Vector Structure"))
  (locals (NewTarget :type "Vector Structure"))
  (bind _returnvalue (`self.GetVelocity` (`self.target_mob`)))
  (bind _returnvalue_2 (`KismetMathLibrary.Vector_Distance` `target point` (`self.shot_location`)))
  (set `self.target_point` (+ `target point` (* _returnvalue (* (/ (`KismetMathLibrary.Vector_Distance` (+ `target point` _returnvalue) (`self.shot_location`)) _returnvalue_2) (/ _returnvalue_2 (/ (`self.speed`) (`GameplayStatics.GetWorldDeltaSeconds`))))))))

(fn `Go To Mob`
  (locals (rate :type "Float (double-precision)" :default 10.0))
  (if (`KismetSystemLibrary.IsValid` (`self.target_mob`))
    (bind _output_get (set `self.shot_location` (`KismetMathLibrary.MakeVector` (+ (.x (`self.shot_location`)) (`self.dx`)) (+ (.y (`self.shot_location`)) (`self.dy`)) (.z (`self.shot_location`)))))
    (`SceneComponent.K2_SetWorldLocation` (`self.CapsuleComponent`) _output_get false false)
    (else
      (`self.K2_DestroyActor`))))

(fn `Hit`
  (`KismetSystemLibrary.PrintString` "destroy actor")
  (`self.K2_DestroyActor`))

(fn `MakeOffset`
  (bind _speed (`self.speed`))
  (bind _returnvalue (- (.x (`self.target_point`)) (.x (`self.shot_location`))))
  (bind _returnvalue_2 (- (.y (`self.target_point`)) (.y (`self.shot_location`))))
  (bind _returnvalue_3 (`KismetMathLibrary.Sqrt` (+ (`KismetMathLibrary.Square` _returnvalue) (`KismetMathLibrary.Square` _returnvalue_2))))
  (set `self.dx` (/ (* _speed _returnvalue) _returnvalue_3))
  (set `self.dy` (/ (* _speed _returnvalue_2) _returnvalue_3)))

(fn `SetShotParams`
  (params (speed :type Integer) (target_mob :type "/Game/Blueprints/Mobs/EnemyMobs/BP_EnemyMob Object Reference") (target_location :type "Vector Structure") (damage :type Integer) (tower_location :type "Vector Structure"))
  (set `self.speed` speed)
  (set `self.target_mob` target_mob)
  (set `self.damage` damage)
  (set `self.shot_location` (`SceneComponent.K2_GetComponentLocation` (`self.Cone`)))
  (set `self.tower location` tower_location)
  (`self.CalculateMobLocation` target_location)
  (`KismetSystemLibrary.PrintString` (`KismetSystemLibrary.GetDisplayName` (`self.target_mob`)))
  (`KismetSystemLibrary.PrintString` (`KismetStringLibrary.Conv_VectorToString` (`self.target_point`)))
  (`self.MakeOffset`))

(fn `TouchEnemyMobHandler`
  (params (Mob :type "Actor Object Reference"))
  (bind _asbp_enemy_mob (cast `/Game/Blueprints/Mobs/EnemyMobs/BP_EnemyMob` Mob))
  (`/Game/Blueprints/Mobs/EnemyMobs/BP_EnemyMob.GetDamage` _asbp_enemy_mob (`self.damage`))
  (`self.Hit`))

(fn `UserConstructionScript`)