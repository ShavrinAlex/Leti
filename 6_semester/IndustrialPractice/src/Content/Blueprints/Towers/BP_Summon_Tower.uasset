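; Summon tower that spawns a squad of AI guardian mobs at formation points around itself.
; BeginPlay creates a placement helper and a cooldown timer, whose expiry sets a flag that Main, polled on Tick, uses to spawn a full batch when below the cap.
; DirectGuards recomputes the formation around a target point and writes each guard's blackboard location.
; Guard-death cleanup is unwired, so the count never drops; cooldown and timer-update functions are stubs.
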(event `self.ReceiveBeginPlay`
  (bind _returnvalue (`SceneComponent.K2_GetComponentLocation` (`self.CapsuleComponent`)))
  (`parent.ReceiveBeginPlay`)
  (bind _returnvalue_2 (`|SpawnActorFromClass` "/Script/TowerDefense.MobPlaceStructure" (`KismetMathLibrary.MakeTransform` _returnvalue) "Undefined" "MultiplyWithRoot" null null))
  (bind _output_get (set `self.mob place struct ref` _returnvalue_2))
  (`MobPlaceStructure.CalculateCoords` _output_get _returnvalue)
  (bind _returnvalue_3 (`|SpawnActorFromClass` "/Script/TowerDefense.SummonTimer" (`KismetMathLibrary.MakeTransform` (0.0 0.0 0.0)) "Undefined" "MultiplyWithRoot" null null))
  (bind _output_get_2 (set `self.summon timer ref` _returnvalue_3))
  (`SummonTimer.SetDelay` _output_get_2 (`self.summon_delay`)))

(event `self.ReceiveTick`
  (params (DeltaSeconds :type "Float (single-precision)"))
  (`parent.ReceiveTick` DeltaSeconds)
  (`self.Main`))

(event `self.summon timer ref.OnTimerExpired`
  (`KismetSystemLibrary.PrintString` "Timer event called in bp" true true (struct :`R` 1.0 :`G` 0.072917 :`B` 0.072917 :`A` 1.0))
  (set `self.is_cooldown_ready` true))

(fn `CheckCooldown`
  (returns (IsCooldownReady :type Boolean))
  (return true))

(fn `CheckGuardDeath`
  (returns (IsGuardDead :type Boolean)))

(fn `DirectGuards`
  (`MobPlaceStructure.CalculateCoords` (`self.mob place struct ref`) (`self.guards_target_point`))
  (for _index (range (`self.max guard count`))
    (bind _returnvalue (`MobPlaceStructure.GetCoordByNumber` (`self.mob place struct ref`) _index))
    (`BlackboardComponent.SetValueAsVector` (`AIBlueprintHelperLibrary.GetBlackboard` (`|GetArrayItem` (`self.guards`) _index)) "TargetLocation" _returnvalue)))

(fn `Main`
  (bind _max_guard_count (`self.max guard count`))
  (if true
    (if (`self.is_cooldown_ready`)
      (`KismetSystemLibrary.PrintString` "update flag")
      (set `self.is_cooldown_ready` false)
      (if (< (`self.current guard count`) _max_guard_count)
        (for _ (range _max_guard_count)
          (`self.Summon Guard`))))))

(fn `Summon Guard`
  (bind _guards (`self.guards`))
  (bind _current_guard_count (`self.current guard count`))
  (bind _returnvalue (`MobPlaceStructure.GetCoordByNumber` (`self.mob place struct ref`) _current_guard_count))
  (bind _returnvalue_2 (`AIBlueprintHelperLibrary.SpawnAIFromClass` "/Game/Blueprints/Mobs/GuardianMobs/BP_GuardianMob.BP_GuardianMob_C" "/Game/Blueprints/Mobs/GuardianMobs/BT_GuardianMob.BT_GuardianMob" _returnvalue (struct) false null))
  (`KismetArrayLibrary.Array_Insert` _guards _returnvalue_2 _current_guard_count)
  (`KismetSystemLibrary.PrintString` (`KismetSystemLibrary.GetDisplayName` (`|GetArrayItem` _guards _current_guard_count)))
  (`KismetSystemLibrary.PrintString` (`KismetStringLibrary.Conv_VectorToString` _returnvalue))
  (`/Engine/EditorBlueprintResources/StandardMacros.IncrementInt` (`self.current guard count`)))

(fn `UpdateTimer`)

(fn `UserConstructionScript`
  (`parent.UserConstructionScript`)
  (set `self.max guard count` 3)
  (set `self.summon_delay` 10))