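; Tower actor for a tower-building game, handling purchase cost, menu, upgrades and selling, with no combat logic.
; The construction script finds the level manager and deducts the tower cost from its money.
; BeginPlay creates a hidden-by-default menu widget, which ClickTowerHandler toggles.
; UpgradeTower only raises level and stored cost, while DeleteTower refunds half that cost, frees its placement spot and destroys the actor.
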(event `self.ReceiveBeginPlay`
  (`self.CreateWidget`))

(event `self.ReceiveTick`
  (params (DeltaSeconds :type "Float (single-precision)")))

(fn `ClickTowerHandler`
  (bind _tower_menu_ref (`self.tower_menu_ref`))
  (if (`self.is_visible_widget`)
    (set `self.is_visible_widget` false)
    (else
      (set `self.is_visible_widget` true)))
  (if (`self.is_visible_widget`)
    (`Widget.SetVisibility` _tower_menu_ref "Visible")
    (`UserWidget.AddToViewport` _tower_menu_ref 0)
    (`KismetSystemLibrary.PrintString` "tower was show")
    (else
      (`Widget.SetVisibility` _tower_menu_ref "Hidden")
      (`KismetSystemLibrary.PrintString` "tower was hide"))))

(fn `CreateWidget`
  (bind _returnvalue (`GameplayStatics.GetPlayerController` 0))
  (set `PlayerController.bEnableClickEvents` true _returnvalue)
  (bind _returnvalue_2 (`|CreateWidget` "/Game/Blueprints/Towers/TowerMenuPopup.TowerMenuPopup_C" _returnvalue))
  (bind _output_get (set `self.tower_menu_ref` _returnvalue_2))
  (`/Game/Blueprints/Towers/TowerMenuPopup.SetTowerRef` _output_get self)
  (set `self.is_visible_widget` false)
  (`KismetSystemLibrary.PrintString` "tower widget created")
  (set `self.level` 1))

(fn `DeleteTower`
  (bind _levelmanagercopy (`self.LevelManagerCopy`))
  (bind _money (`LevelManager.money` _levelmanagercopy))
  (set `/Game/Blueprints/Towers/BP_Tower_Place.is_tower_placed` false (`self.Tower Place Ref`))
  (set `LevelManager.money` (+ _money (/ (`self.tower_cost`) 2)) _levelmanagercopy)
  (`KismetSystemLibrary.PrintString` (`KismetStringLibrary.Conv_IntToString` _money))
  (`KismetSystemLibrary.PrintString` "tower deleted")
  (`Widget.RemoveFromParent` (`self.tower_menu_ref`))
  (`self.K2_DestroyActor`))

(fn `SetTowerPlaceRef`
  (params (TowerPlaceRef :type "/Game/Blueprints/Towers/BP_Tower_Place Object Reference"))
  (set `self.Tower Place Ref` TowerPlaceRef))

(fn `UpgradeTower`
  (params (upgrade_type :type String))
  (`/Engine/EditorBlueprintResources/StandardMacros.IncrementInt` (`self.level`)
    (:`  `
      (set `self.tower_cost` (`KismetMathLibrary.FTrunc` (* (`self.tower_cost`) 1.5))))))

(fn `UserConstructionScript`
  (bind _outactors (`GameplayStatics.GetAllActorsOfClass` "/Game/Blueprints/LevelManager/BP_LevelManager.BP_LevelManager_C"))
  (bind _output_get (set `self.LevelManagerCopy` (`|GetArrayItem` _outactors)))
  (set `LevelManager.money` (- (`LevelManager.money` _output_get) (`self.tower_cost`)) _output_get))