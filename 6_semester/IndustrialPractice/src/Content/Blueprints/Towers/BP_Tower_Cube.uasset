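; BP_Tower_Cube is the cube tower Blueprint, a child tower that sets its own cost, creates a widget on BeginPlay and handles clicks on its mesh.
; UpgradeTower runs the parent upgrade, then SetTowerTexture swaps the static mesh by upgrade type, despite its name.
; Only level 2 has meshes, one for each of two branches; other levels or types fail, with results reported through debug prints.
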(event `self.ReceiveBeginPlay`
  (`parent.ReceiveBeginPlay`)
  (`self.CreateWidget`))

(event `self.Tower.OnClicked`
  (params (TouchedComponent :type "PrimitiveComponent Object Reference") (ButtonPressed :type "Key Structure"))
  (`self.ClickTowerHandler`))

(fn `NewFunction_0`)

(fn `NewFunction_1`)

(fn `SetTowerTexture`
  (params (level :type Integer) (upgrade_type :type String))
  (returns (is_succes :type Boolean))
  (bind _tower (`self.Tower`))
  (switch `int` level
    (:`Default`
      (`KismetSystemLibrary.PrintString` "Max level!"))
    (:`2`
      (switch `string` upgrade_type
        (:`Default`
          (`KismetSystemLibrary.PrintString` "No such tower"))
        (:`first`
          (`StaticMeshComponent.SetStaticMesh` _tower "/Engine/EngineMeshes/Cylinder.Cylinder")
          (return true))
        (:`second`
          (`StaticMeshComponent.SetStaticMesh` _tower "/Engine/VREditor/BasicMeshes/SM_Cube_03.SM_Cube_03")
          (return true)))))
  (return false))

(fn `UpgradeTower`
  (params (upgrade_type :type String))
  (`parent.UpgradeTower` upgrade_type)
  (`KismetSystemLibrary.PrintString` (`KismetStringLibrary.BuildString_Int` upgrade_type "" (`self.level`)))
  (bind _is_succes (`self.SetTowerTexture` (`self.level`) (`local.upgrade_type`)))
  (if _is_succes
    (`KismetSystemLibrary.PrintString` "Success upgrade")
    (else
      (`KismetSystemLibrary.PrintString` "Tower cannot be upgraded"))))

(fn `UserConstructionScript`
  (set `self.tower_cost` 100)
  (`parent.UserConstructionScript`))