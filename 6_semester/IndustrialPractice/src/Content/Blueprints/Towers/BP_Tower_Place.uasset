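; BP_Tower_Place is a clickable tower slot that opens a popup for choosing a tower.
; On BeginPlay it enables mouse clicks and cursor, creates a TowerChoosePopup widget and passes itself to it as a reference.
; Clicking the TowerPlace component toggles the popup and, on opening, stores a location just above the slot in LocationVector.
; If a tower is already placed, clicking only prints a message.
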(event `self.ReceiveBeginPlay`
  (`self.CreateWidget`))

(event `self.tower place.OnClicked`
  (params (TouchedComponent :type "PrimitiveComponent Object Reference") (ButtonPressed :type "Key Structure"))
  (bind _towerplacemenuref (`self.TowerPlaceMenuRef`))
  (if (`self.is_tower_placed`)
    (`KismetSystemLibrary.PrintString` "tower already placed")
    (else
      (if (`self.is_visible_widget`)
        (set `self.is_visible_widget` false)
        (else
          (set `self.is_visible_widget` true)))
      (if (`self.is_visible_widget`)
        (`Widget.SetVisibility` _towerplacemenuref "Visible")
        (`UserWidget.AddToViewport` _towerplacemenuref 0)
        (set `self.location_vector` (+ (`SceneComponent.K2_GetComponentLocation` (`self.tower place`)) (0.0 0.0 1.0)))
        (else
          (`Widget.SetVisibility` _towerplacemenuref "Hidden"))))))

(fn `CreateWidget`
  (bind _returnvalue (`GameplayStatics.GetPlayerController` 0))
  (set `PlayerController.bEnableClickEvents` true _returnvalue)
  (set `PlayerController.bShowMouseCursor` true _returnvalue)
  (bind _returnvalue_2 (`|CreateWidget` "/Game/Blueprints/Towers/TowerChoosePopup.TowerChoosePopup_C" _returnvalue))
  (bind _output_get (set `self.TowerPlaceMenuRef` _returnvalue_2))
  (`/Game/Blueprints/Towers/TowerChoosePopup.SetTowerPlaceRef` _output_get self)
  (set `self.is_visible_widget` false))

(fn `UserConstructionScript`)