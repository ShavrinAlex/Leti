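; Sphere tower Blueprint, a child of a tower parent class, with its cost set in the Construction Script.
; It creates a widget on BeginPlay and forwards clicks on its Sphere mesh to the tower click handler.
; UpgradeTower runs parent logic, then SetTowerTexture swaps the mesh to a cone or cylinder at level two by upgrade type.
; SetTowerTexture always returns false, so even successful swaps print the failure message.
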(event `self.ReceiveBeginPlay`
  (`parent.ReceiveBeginPlay`)
  (`self.CreateWidget`))

(event `self.Sphere.OnClicked`
  (params (TouchedComponent :type "PrimitiveComponent Object Reference") (ButtonPressed :type "Key Structure"))
  (`self.ClickTowerHandler`))

(fn `NewFunction_0`)

(fn `SetTowerTexture`
  (params (level :type Integer) (upgrade_type :type String))
  (returns (is_success :type Boolean))
  (bind _sphere (`self.Sphere`))
  (switch `int` level
    (:`Default`
      (`KismetSystemLibrary.PrintString` "Max level!"))
    (:`2`
      (switch `string` upgrade_type
        (:`Default`
          (`KismetSystemLibrary.PrintString` "No such tower"))
        (:`first`
          (`StaticMeshComponent.SetStaticMesh` _sphere "/Engine/BasicShapes/Cone.Cone")
          (return false))
        (:`second`
          (`StaticMeshComponent.SetStaticMesh` _sphere "/Engine/BasicShapes/Cylinder.Cylinder")
          (return false)))))
  (return false))

(fn `UpgradeTower`
  (params (upgrade_type :type String))
  (locals (info_string :type String))
  (`parent.UpgradeTower` upgrade_type)
  (`KismetSystemLibrary.PrintString` (`KismetStringLibrary.BuildString_Int` upgrade_type "" (`self.level`)))
  (bind _is_success (`self.SetTowerTexture` (`self.level`) (`local.upgrade_type`)))
  (if _is_success
    (`KismetSystemLibrary.PrintString` "Success upgrade")
    (else
      (`KismetSystemLibrary.PrintString` "Tower cannot be upgraded"))))

(fn `UserConstructionScript`
  (set `self.tower_cost` 120)
  (`parent.UserConstructionScript`))